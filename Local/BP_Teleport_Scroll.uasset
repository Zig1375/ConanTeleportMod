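; Teleport scroll item that moves its user to the nearest BP_PL_Teleport_1 they own.
; On use, the server scans all teleports, measuring ownership and distance from player controller 0's pawn rather than the invoking character.
; It animates the chosen teleport around a short delay, moves the invoker to its direction indicator, decrements or removes the stack, then logs the loss.
; Without an owned teleport, it shows a failure notification.
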(event `self.OnUseItem_Implementation`
  (params (InvokingCharacter :type "ConanCharacter Object Reference"))
  (bind _returnvalue (`self.GetIntStat` "StackSize"))
  (bind _returnvalue_2 (`self.GetOwnerInventory`))
  (if (or (`KismetSystemLibrary.IsDedicatedServer`) (`KismetSystemLibrary.IsServer`))
    (bind (_founded _result) (`self.GetNearestTeleport`))
    (if _founded
      ;[1 1 1] Teleport
      (`/Game/Mods/Teleport/BP_PL_Teleport_1.AnimateSelfTeleport` _result 0.0 1.0 false)
      (`KismetSystemLibrary.Delay` 0.5)
      (`Actor.K2_SetActorLocation` InvokingCharacter (`SceneComponent.K2_GetComponentLocation` (`/Game/Systems/Building/Placeables/BP_Master_Placeables.DirectionIndicatorMesh` _result)) false false)
      (`/Game/Mods/Teleport/BP_PL_Teleport_1.AnimateSelfTeleport` _result 1.0 0.0 true)
      (`|ExecutionSequence`
        (:`then_0`
          ;[1 1 1] Consume item from item stack. If empty, remove item.
          (if (<= _returnvalue 1)
            (`ItemInventory.RemoveItem` _returnvalue_2 (`ItemInventory.GetItemIndex` _returnvalue_2 self))
            (else
              (`self.SetIntStat` "StackSize" (- _returnvalue 1)))))
        (:`then_1`
          ;[1 1 1] Lootlog
          (bind _asbase_game_hud (cast `/Game/UI/HUD/BaseGameHUD` (`self.GetOwner`)))
          (`ConanHUD.AddItemToLootLog` _asbase_game_hud (`self.TemplateID`) -1 0)))
      (else
        ;[1 1 1] Teleport not found
        (`ConanCharacter.ClientHUDShowNotification` InvokingCharacter "Teleports not found" false)))))

(fn `CanUseItem`
  (params (invokingCharacter :type "ConanCharacter Object Reference"))
  (returns (ReturnValue :type Boolean))
  (return true))

(fn `CheckTeleportOwner`
  (params (target :type "/Game/Systems/Building/Placeables/BP_Master_Placeables Object Reference") (Instigator :type "PlayerController Object Reference"))
  (returns (Instigator_Out :type "PlayerController Object Reference") (HitIndex_Out :type Integer) (IsOwner :type Boolean))
  (return Instigator 0 (`BuildableBase.IsOwner` target (`Controller.K2_GetPawn` Instigator) false)))

(fn `GetNearestTeleport`
  (returns (founded :type Boolean) (result :type "/Game/Mods/Teleport/BP_PL_Teleport_1 Object Reference"))
  (locals (Distance :type "Float (double-precision)" :default 0.0) (Teleport :type "/Game/Mods/Teleport/BP_PL_Teleport_1 Object Reference"))
  (bind _returnvalue (`GameplayStatics.GetPlayerController` 0))
  (set `local.Distance` 999999999.0)
  (bind _outactors (`GameplayStatics.GetAllActorsOfClass` "/Game/Mods/Teleport/BP_PL_Teleport_1.BP_PL_Teleport_1_C"))
  (for _array_element _outactors
    (bind (_instigator_out _hitindex_out _isowner) (`self.CheckTeleportOwner` _array_element _returnvalue))
    (if _isowner
      (bind _returnvalue_2 (`KismetMathLibrary.VSize` (- (`Actor.K2_GetActorLocation` (`Controller.K2_GetPawn` _returnvalue)) (`Actor.K2_GetActorLocation` _array_element))))
      (if (> (`local.Distance`) _returnvalue_2)
        (set `local.Distance` _returnvalue_2)
        (set `local.Teleport` _array_element))))
  (return (< (`local.Distance`) 999999999.0) (`local.Teleport`)))